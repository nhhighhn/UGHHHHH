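; BP_HealthRegen is a reusable health pickup that restores a random amount of health to the actor that overlaps it.
; On overlap it calls RegenerateHealth on that actor's BP_HealthComp, and is consumed only if the call returns true.
; Consumption hides the cross, disables trigger collision and attaches a Niagara effect to the actor, then restores both cross and trigger after a brief delay.
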(event `self.Overlapped`
  (params (OtherActor :type "Actor Object Reference"))
  (bind _regen_successful (`/Game/Components/BP_HealthComp.RegenerateHealth` (`self.GetComponentByClass` OtherActor "/Game/Components/BP_HealthComp.BP_HealthComp_C") (`KismetMathLibrary.RandomFloatInRange` 10.0 50.0)))
  (if _regen_successful
    (`self.Consumed` OtherActor)))

(event `Consumed`
  (params (Target :type "Actor Object Reference"))
  (`SceneComponent.SetVisibility` (`self.Cross`) false true)
  (`PrimitiveComponent.SetCollisionEnabled` (`self.Trigger`) "NoCollision")
  (`NiagaraFunctionLibrary.SpawnSystemAttached` null (`Actor.RootComponent` Target) "None" (0.0 0.0 0.0) (struct) "SnapToTarget")
  (`KismetSystemLibrary.Delay` 0.2)
  (`SceneComponent.SetVisibility` (`self.Cross`) true true)
  (`PrimitiveComponent.SetCollisionEnabled` (`self.Trigger`) "QueryAndPhysics"))

(fn `UserConstructionScript`
  (`parent.UserConstructionScript`))